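; BP_BezierActor is a construction-time actor that lays out copies of a chosen actor class along a Bezier curve in its local XZ plane.
; The Construction Script packs each control point's X and Z with a matching stroke scale into one vector, then feeds the list to BezierCurve.
; Each returned point spawns a child actor component, using the third channel as uniform scale for variable stroke width.
; The event graph holds no runtime logic.
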(fn `UserConstructionScript`
  (`KismetArrayLibrary.Array_Clear` (`self.Loc2D_with_stroke`))
  (for (_array_element _array_index) (`self.Param`)
    (`KismetArrayLibrary.Array_AddUnique` (`self.Loc2D_with_stroke`) (`KismetMathLibrary.MakeVector` (.x _array_element) (.z _array_element) (`|GetArrayItem` (`self.Stroke Scale`) _array_index))))
  (bind _returnvalue (`self.BezierCurve` (`self.Loc2D_with_stroke`)))
  (for _array_element_2 _returnvalue
    (bind _returnvalue_2 (`AddComponent|NODE_AddChildActorComponent-0` :`RelativeTransform` (`KismetMathLibrary.MakeTransform` (`KismetMathLibrary.MakeVector` (.x _array_element_2) 0.0 (.y _array_element_2)) (struct) (`KismetMathLibrary.MakeVector` (.z _array_element_2) (.z _array_element_2) (.z _array_element_2)))))
    (`ChildActorComponent.SetChildActorClass` _returnvalue_2 (`self.In Class`))))
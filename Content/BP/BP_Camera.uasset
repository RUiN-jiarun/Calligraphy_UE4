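; Camera rig Blueprint that exposes custom events to rotate, zoom and pan a spring arm camera, with no input handling of its own.
; CE_Rotation adds unclamped pitch to the SpringArm, then zeroes roll and clamps yaw to a fixed range.
; CE_Scale clamps arm length to caller-supplied limits.
; CE_Transform moves Root along the arm's target right and forward vectors, so pans follow the view direction, pitch included.
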(event `CE_Rotation`
  (params (Horizontal :type "Float (double-precision)") (Vertical :type "Float (double-precision)") (Interpolation :type "Float (double-precision)"))
  (`SceneComponent.K2_AddRelativeRotation` (`self.SpringArm`) (`KismetMathLibrary.MakeRotator` 0.0 (* Vertical Interpolation)) false false)
  (`SceneComponent.K2_SetRelativeRotation` (`self.SpringArm`) (`KismetMathLibrary.MakeRotator` 0.0 (.pitch (`SceneComponent.RelativeRotation` (`self.SpringArm`))) (`KismetMathLibrary.FClamp` (+ (* Horizontal Interpolation) (.yaw (`SceneComponent.RelativeRotation` (`self.SpringArm`)))) -70.0 70.0)) false false))

(event `CE_Scale`
  (params (Param :type "Float (double-precision)") (Interpolation :type "Float (double-precision)") (MinDistance :type "Float (double-precision)") (MaxDistance :type "Float (double-precision)"))
  (bind _springarm (`self.SpringArm`))
  (set `SpringArmComponent.TargetArmLength` (`KismetMathLibrary.FClamp` (+ (* Param Interpolation) (`SpringArmComponent.TargetArmLength` _springarm)) MinDistance MaxDistance) _springarm))

(event `CE_Transform`
  (params (Horizontal :type "Float (double-precision)") (Vertical :type "Float (double-precision)") (Interpolation_X :type "Float (double-precision)") (Interpolation_Y :type "Float (double-precision)"))
  (bind _returnvalue (`SpringArmComponent.GetTargetRotation` (`self.SpringArm`)))
  (`SceneComponent.K2_SetRelativeLocation` (`self.Root`) (+ (`SceneComponent.RelativeLocation` (`self.Root`)) (+ (* (`KismetMathLibrary.GetRightVector` _returnvalue) (* Horizontal Interpolation_X)) (* (`KismetMathLibrary.GetForwardVector` _returnvalue) (* Vertical Interpolation_Y)))) false false))

(fn `UserConstructionScript`)
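; BP_SimpleBezier is an actor for following a quadratic Bézier curve from its spawn location, through a control anchor, to an end point.
; BeginPlay converts points to world space and starts TimelineLerp after a delay; movement and trail drawing sit in a disconnected Timeline_Lerp update.
; Nested lerps compute location, and finite differences give tangent-facing rotation.
; DrawCurve and an optional construction-script preview sample the curve as debug lines.
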(event `self.ReceiveBeginPlay`
  (set `self.Start` (`self.K2_GetActorLocation`))
  (`self.UpdateToWorldVector` (`self.ControlAnchor`))
  (`self.UpdateToWorldVector` (`self.End`))
  (`KismetSystemLibrary.Delay` 0.5)
  (`TimelineComponent.PlayFromStart` (`self.Timeline_Lerp`)))

(fn `DrawCurve`
  (`self.DrawCurveForSeconds` 2.0))

(fn `DrawCurveForSeconds`
  (params (InDuration :type "Float (double-precision)" :default 2.0))
  (locals (Temp_DebugStart :type "Vector Structure" :default (0.0 0.0 0.0)) (Temp_Time :type "Float (double-precision)") (Temp_DebugEnd :type "Vector Structure" :default (0.0 0.0 0.0)))
  (set `local.Temp_DebugStart` (`self.K2_GetActorLocation`))
  (while (`KismetMathLibrary.InRange_FloatFloat` (`local.Temp_Time`))
    (`|ExecutionSequence`
      (:`then_0`
        (bind _output_get (set `local.Temp_DebugEnd` (`KismetMathLibrary.TransformLocation` (`self.GetTransform`) (`self.GetLocationBezier` (`self.Start`) (`self.ControlAnchor`) (`self.End`) (`local.Temp_Time`)))))
        (`KismetSystemLibrary.DrawDebugLine` (`local.Temp_DebugStart`) _output_get (struct :`R` 1.0 :`A` 1.0) InDuration 5.0)
        (set `local.Temp_DebugStart` (`local.Temp_DebugEnd`)))
      (:`then_1`
        (set `local.Temp_Time` (+ (`local.Temp_Time`) 0.01))))))

(fn `GetLocationBezier`
  (params (StartPoint :type "Vector Structure") (AnchorPoint :type "Vector Structure") (EndPoint :type "Vector Structure") (Time :type "Float (double-precision)"))
  (returns (RenturnValue :type "Vector Structure"))
  (locals (Temp_A :type "Vector Structure" :default (0.0 0.0 0.0)) (Temp_B :type "Vector Structure" :default (0.0 0.0 0.0)))
  (`|ExecutionSequence`
    (:`then_0`
      (set `local.Temp_A` (`KismetMathLibrary.VLerp` StartPoint AnchorPoint Time))
      (set `local.Temp_B` (`KismetMathLibrary.VLerp` AnchorPoint EndPoint Time)))
    (:`then_1`
      (return (`KismetMathLibrary.VLerp` (`local.Temp_A`) (`local.Temp_B`) Time)))))

(fn `GetRotationBezier`
  (params (StartPoint :type "Vector Structure") (AnchorPoint :type "Vector Structure") (EndPoint :type "Vector Structure") (Time :type "Float (double-precision)"))
  (returns (RenturnValue :type "Rotator Structure"))
  (locals (Temp_Current :type "Vector Structure" :default (0.0 0.0 0.0)))
  (bind _returnvalue (+ Time -0.001))
  (set `local.Temp_Current` (`self.GetLocationBezier` StartPoint AnchorPoint EndPoint Time))
  (if (`KismetMathLibrary.InRange_FloatFloat` _returnvalue)
    (return (`KismetMathLibrary.Conv_VectorToRotator` (`KismetMathLibrary.Normal` (- (`local.Temp_Current`) (`self.GetLocationBezier` StartPoint AnchorPoint EndPoint _returnvalue)))))
    (else
      (return (`KismetMathLibrary.Conv_VectorToRotator` (`KismetMathLibrary.Normal` (- (`self.GetLocationBezier` StartPoint AnchorPoint EndPoint (+ Time 0.001)) (`local.Temp_Current`))))))))

(fn `UpdateToWorldVector`
  (params (InVec :type "Vector Structure (by ref)"))
  (`|VariableSetRef` InVec (`KismetMathLibrary.TransformLocation` (`self.GetTransform`) InVec)))

(fn `UserConstructionScript`
  (if (`self.bDebugCurveConstruction`)
    (`self.DrawCurveForSeconds` 0.02)))
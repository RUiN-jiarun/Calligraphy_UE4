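; Cubic Bezier actor that defines a curved path with varying stroke thickness, meant for moving itself along it.
; Nested lerps evaluate location and thickness, and sampling a nearby point gives tangent rotation.
; BeginPlay converts points to world space and starts a timeline after a delay, but the update that moves the actor and draws its trail sits under a separately named, never-run timeline.
; Debug helpers draw the curve, optionally during construction.
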(event `self.ReceiveBeginPlay`
  (set `self.Start` (`self.K2_GetActorLocation`))
  (`self.UpdateToWorldVector` (`self.StartAnchor`))
  (`self.UpdateToWorldVector` (`self.EndAnchor`))
  (`self.UpdateToWorldVector` (`self.End`))
  (`KismetSystemLibrary.Delay` 0.75)
  (`TimelineComponent.PlayFromStart` (`self.Timeline_Lerp`)))

(fn `DrawCurve`
  (`self.DrawCurveForSeconds` 2.0))

(fn `DrawCurveForSeconds`
  (params (InDuration :type "Float (double-precision)" :default 2.0))
  (locals (Temp_DebugStart :type "Vector Structure" :default (0.0 0.0 0.0)) (Temp_Time :type "Float (double-precision)") (Temp_DebugEnd :type "Vector Structure" :default (0.0 0.0 0.0)))
  (set `local.Temp_DebugStart` (`self.K2_GetActorLocation`))
  (while (`KismetMathLibrary.InRange_FloatFloat` (`local.Temp_Time`))
    (`|ExecutionSequence`
      (:`then_0`
        (bind _output_get (set `local.Temp_DebugEnd` (`KismetMathLibrary.TransformLocation` (`self.GetTransform`) (`self.GetLocationBezier` (`self.Start`) (`self.StartAnchor`) (`self.EndAnchor`) (`self.End`) (`local.Temp_Time`)))))
        (`KismetSystemLibrary.DrawDebugLine` (`local.Temp_DebugStart`) _output_get (struct :`R` 1.0 :`A` 1.0) InDuration (`self.GetStrokeBezier` (`self.StartStroke`) (`self.StartAnchorStroke`) (`self.EndAnchorStroke`) (`self.EndStroke`) (`local.Temp_Time`)))
        (set `local.Temp_DebugStart` (`local.Temp_DebugEnd`)))
      (:`then_1`
        (set `local.Temp_Time` (+ (`local.Temp_Time`) 0.01))))))

(fn `GetLocationBezier`
  (params (StartPoint :type "Vector Structure") (AnchorStart :type "Vector Structure") (AnchorEnd :type "Vector Structure") (EndPoint :type "Vector Structure") (Time :type "Float (double-precision)"))
  (returns (RenturnValue :type "Vector Structure"))
  (locals (Temp_A :type "Vector Structure" :default (0.0 0.0 0.0)) (Temp_B :type "Vector Structure" :default (0.0 0.0 0.0)) (Temp_C :type "Vector Structure") (Temp_D :type "Vector Structure" :default (0.0 0.0 0.0)) (Temp_E :type "Vector Structure" :default (0.0 0.0 0.0)))
  (`|ExecutionSequence`
    (:`then_0`
      (set `local.Temp_A` (`KismetMathLibrary.VLerp` StartPoint AnchorStart Time))
      (set `local.Temp_B` (`KismetMathLibrary.VLerp` AnchorStart AnchorEnd Time))
      (set `local.Temp_C` (`KismetMathLibrary.VLerp` AnchorEnd EndPoint Time)))
    (:`then_1`
      (set `local.Temp_D` (`KismetMathLibrary.VLerp` (`local.Temp_A`) (`local.Temp_B`) Time))
      (set `local.Temp_E` (`KismetMathLibrary.VLerp` (`local.Temp_B`) (`local.Temp_C`) Time)))
    (:`then_2`
      (return (`KismetMathLibrary.VLerp` (`local.Temp_D`) (`local.Temp_E`) Time)))))

(fn `GetRotationBezier`
  (params (StartPoint :type "Vector Structure") (AnchorStart :type "Vector Structure") (AnchorEnd :type "Vector Structure") (EndPoint :type "Vector Structure") (Time :type "Float (double-precision)"))
  (returns (RenturnValue :type "Rotator Structure"))
  (locals (Temp_Current :type "Vector Structure" :default (0.0 0.0 0.0)))
  (bind _returnvalue (+ Time -0.001))
  (set `local.Temp_Current` (`self.GetLocationBezier` StartPoint AnchorStart AnchorEnd EndPoint Time))
  (if (`KismetMathLibrary.InRange_FloatFloat` _returnvalue)
    (return (`KismetMathLibrary.Conv_VectorToRotator` (`KismetMathLibrary.Normal` (- (`local.Temp_Current`) (`self.GetLocationBezier` StartPoint AnchorStart AnchorEnd EndPoint _returnvalue)))))
    (else
      (return (`KismetMathLibrary.Conv_VectorToRotator` (`KismetMathLibrary.Normal` (- (`self.GetLocationBezier` StartPoint AnchorStart AnchorEnd EndPoint (+ Time 0.001)) (`local.Temp_Current`))))))))

(fn `GetStrokeBezier`
  (params (StartPointStroke :type "Float (double-precision)") (AnchorStartStroke :type "Float (double-precision)") (AnchorEndStroke :type "Float (double-precision)") (EndPointStroke :type "Float (double-precision)") (Time :type "Float (double-precision)"))
  (returns (RenturnValue :type "Float (double-precision)"))
  (locals (Temp_A :type "Float (double-precision)") (Temp_B :type "Float (double-precision)") (Temp_C :type "Float (double-precision)") (Temp_D :type "Float (double-precision)") (Temp_E :type "Float (double-precision)"))
  (`|ExecutionSequence`
    (:`then_0`
      (set `local.Temp_A` (`KismetMathLibrary.Lerp` StartPointStroke AnchorStartStroke Time))
      (set `local.Temp_B` (`KismetMathLibrary.Lerp` AnchorStartStroke AnchorEndStroke Time))
      (set `local.Temp_C` (`KismetMathLibrary.Lerp` AnchorEndStroke EndPointStroke Time)))
    (:`then_1`
      (set `local.Temp_D` (`KismetMathLibrary.Lerp` (`local.Temp_A`) (`local.Temp_B`) Time))
      (set `local.Temp_E` (`KismetMathLibrary.Lerp` (`local.Temp_B`) (`local.Temp_C`) Time)))
    (:`then_2`
      (return (`KismetMathLibrary.Lerp` (`local.Temp_D`) (`local.Temp_E`) Time)))))

(fn `UpdateToWorldVector`
  (params (InVec :type "Vector Structure (by ref)"))
  (`|VariableSetRef` InVec (`KismetMathLibrary.TransformLocation` (`self.GetTransform`) InVec)))

(fn `UserConstructionScript`
  (if (`self.bDebugCurveConstruction`)
    (`self.DrawCurveForSeconds` 0.1)))